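; Random firework launcher prop that fires BaseFireworksShell projectiles with randomized looks and behavior, then destroys itself.
; FireShellRandom picks among eleven arrow components for the launch transform, adds angular jitter, and randomizes burst effect, flare color, timing and speeds.
; A retriggerable delay removes the launcher after the last shot.
; LaunchTimedShell counts down launches, then clears a timer named LaunchShell, which differs from its own name.
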(event `FireShellRandom`
  (bind _burstparticlesystems (`self.BurstParticleSystems`))
  ;[1 1 1] Launch the shell!
  (`|SpawnActorFromClass` "/Game/CustomContent/UGC2349758790/Fireworks/Props/BaseFireworksShell.BaseFireworksShell_C" (`KismetMathLibrary.MakeTransform` (.location (`SceneComponent.K2_GetComponentToWorld` (select `int` (`KismetMathLibrary.RandomInteger` 11) :`0` (`self.Arrow`) :`1` (`self.Arrow6`) :`2` (`self.Arrow2`) :`3` (`self.Arrow3`) :`4` (`self.Arrow4`) :`5` (`self.Arrow5`) :`6` (`self.Arrow1`) :`7` (`self.Arrow7`) :`8` (`self.Arrow8`) :`9` (`self.Arrow9`) :`10` (`self.Arrow10`) :!type "SceneComponent Object Reference"))) (`KismetMathLibrary.ComposeRotators` (.rotation (`SceneComponent.K2_GetComponentToWorld` (select `int` (`KismetMathLibrary.RandomInteger` 11) :`0` (`self.Arrow`) :`1` (`self.Arrow6`) :`2` (`self.Arrow2`) :`3` (`self.Arrow3`) :`4` (`self.Arrow4`) :`5` (`self.Arrow5`) :`6` (`self.Arrow1`) :`7` (`self.Arrow7`) :`8` (`self.Arrow8`) :`9` (`self.Arrow9`) :`10` (`self.Arrow10`) :!type "SceneComponent Object Reference"))) (`KismetMathLibrary.MakeRotator` (`KismetMathLibrary.RandomFloatInRange` (* (`self.RandomAngle`) -1.0) (`self.RandomAngle`)) (`KismetMathLibrary.RandomFloatInRange` (* (`self.RandomAngle`) -1.0) (`self.RandomAngle`)) (`KismetMathLibrary.RandomFloatInRange` (* (`self.RandomAngle`) -1.0) (`self.RandomAngle`))))) "AlwaysSpawn" "OverrideRootScale" null (`KismetMathLibrary.RandomFloatInRange` 1800.0 2400.0) (`KismetMathLibrary.RandomFloatInRange` 800.0 1200.0) (`KismetMathLibrary.RandomFloatInRange` 6000.0 8500.0) (`self.MinLaunchVelocity`) (`KismetMathLibrary.RandomFloatInRange` 5.0 6.0) (`KismetMathLibrary.RandomFloatInRange` 4.0 5.0) (`KismetMathLibrary.RandomFloatInRange` 6.0 8.0) (`KismetMathLibrary.RandomFloatInRange` 4.5 5.5) (`|GetArrayItem` _burstparticlesystems (`KismetMathLibrary.RandomInteger` (`KismetArrayLibrary.Array_Length` _burstparticlesystems))) (`self.ShellParticleSystem`) (`KismetMathLibrary.RandomIntegerInRange` 1 3) (`KismetMathLibrary.RandomFloatInRange` 0.2 0.5) (select `int` (`KismetMathLibrary.RandomIntegerInRange` 0 5) :`0` (struct :`R` 1.0 :`G` 1.0 :`B` 1.0 :`A` 1.0) :`1` (struct :`R` 1.0 :`A` 1.0) :`2` (struct :`G` 1.0 :`A` 1.0) :`3` (struct :`G` 0.014808 :`B` 1.0 :`A` 1.0) :`4` (struct :`R` 0.825809 :`G` 1.0 :`A` 1.0) :`5` (struct :`R` 1.0 :`B` 0.84287 :`A` 1.0) :!type "LinearColor Structure") (`self.ShellTailColor`) (`self.UseShapedBurst`) (`self.UseShellSmoke`) (`self.UseBurstSmoke`) (`self.BurstSparkleMultiplier`) (`self.ShellSparkleMultiplier`) (`self.BurstStarMultiplier`) (`self.ShapedBurstActorMesh`) (`self.RandomRotation`) null) ; Spawn a shell projectile and pass settings through
  (`KismetSystemLibrary.RetriggerableDelay` 5.0)
  (`self.K2_DestroyActor`))

(fn `LaunchTimedShell`
  (if (!= (`self.NumberOfLaunches`) 0)
    (set `self.NumberOfLaunches` (- (`self.NumberOfLaunches`) 1))
    (`self.FireShellRandom`)
    (else
      (`KismetSystemLibrary.K2_ClearTimer` null "LaunchShell"))))

(fn `UserConstructionScript`
  (`parent.UserConstructionScript`))